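; BP_CoopGameMode is a co-op game mode Blueprint that supplies spawn transforms for bots.
; FindBotSpawnTransform gathers all PlayerPawn actors and ShooterBotWaypoint actors, keeping waypoints that sit beyond a minimum distance from every player.
; It picks one valid waypoint at random and raises it in Z because the points stick into terrain, returning false when none qualify.
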(fn ConstructionScript)

(fn FindBotSpawnTransform
  (bind _validpoints (LocalVariables|GetValidPoints))
  (bind _outactors (Actor|GetAllActorsOfClass "/Game/Blueprints/PlayerPawn.PlayerPawn_C"))
  (LocalVariables|SetPlayers _outactors) ; Cache
  (bind _outactors_2 (Actor|GetAllActorsOfClass "/Script/prototype.ShooterBotWaypoint"))
  (for _array_element _outactors_2
    (LocalVariables|SetbValidSpawnPoint true)
    (bind _array_element_2 (Utilities|Array|ForEachLoopwithBreak (LocalVariables|GetPlayers) :!label _label)
      (:LoopBody
        (if (not (> (Math|Vector|VectorLength (- (Transformation|GetActorLocation _array_element_2) (Transformation|GetActorLocation _array_element))) 1e+02))
          (LocalVariables|SetbValidSpawnPoint false) ; Invalid, skip for consideration.
          (goto _label Break)))
      (:Completed
        (if (LocalVariables|GetbValidSpawnPoint)
          (Utilities|Array|Add (LocalVariables|GetValidPoints) _array_element)))))
  (if (> (Utilities|Array|Length _validpoints) 0)
    (LocalVariables|SetBestSpawn (Utilities|Array|Get(acopy) _validpoints (Math|Random|RandomIntegerinRange 0 (- (Utilities|Array|Length _validpoints) 1))))
    (return (Math|Transform|MakeTransform (+ (Transformation|GetActorLocation (LocalVariables|GetBestSpawn)) "0, 0,80.000000")) (!= (LocalVariables|GetBestSpawn) 0))
    (else
      (return "" false) ; No valid points.
    )))